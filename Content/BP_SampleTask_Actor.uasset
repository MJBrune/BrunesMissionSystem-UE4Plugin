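; Sample mission task actor that completes its task, and optionally the whole mission, through player interaction by overlap.
; On registration with a mission it shows its map icon and binds to the parent task's completion event.
; When a JPCharacter overlaps it while registered, it optionally completes the task, then destroys itself.
; If set to end the mission with the task, it completes the parent mission with the task's failure state and destroys itself.
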(event `self.ReceiveActorBeginOverlap`
  (params (OtherActor :type "Actor Object Reference"))
  (if (`self.bIsRegisteredWithMission`)
    (cast `JPCharacter` OtherActor)
    (if (`self.CompleteTaskOnOverlap`)
      (`BruMissionTask.CompleteTask` (`self.ParentMissionTask`) false))
    (`self.K2_DestroyActor`)))

(event `self.OnRegisterMissionActor`
  (`parent.OnRegisterMissionActor`)
  (add `BruMissionTask.OnTaskCompleted` (`self.ParentMissionTask`) (delegate `OnTaskCompleted`))
  (`MapIconComponent.SetIconVisible` (`self.MapIcon`) true))

(event `OnTaskCompleted`
  (params (FailedTask :type "BruMissionTask Object Reference") (bTaskHasFailed :type Boolean))
  (if (`self.CompleteMissionWhenTaskCompletes`)
    (`BruMissionMetaData.CompleteMission` (`self.ParentMission`) bTaskHasFailed)
    (`self.K2_DestroyActor`)))

(fn `UserConstructionScript`)