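; BP_MissionActivator is a one-shot trigger volume that starts a mission and one of its tasks when the player walks into it.
; On overlap by a JPCharacter with a JPPlayerController, it asks that controller's MissionManager to activate MissionClass.
; If activation returns nothing valid, it looks up the active mission of that class instead.
; Either way it activates MisionTaskClass with a notify broadcast, then destroys itself.
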(event `self.Trigger.OnComponentBeginOverlap`
  (params (OverlappedComponent :type "PrimitiveComponent Object Reference") (OtherActor :type "Actor Object Reference") (OtherComp :type "PrimitiveComponent Object Reference") (OtherBodyIndex :type Integer) (bFromSweep :type Boolean) (SweepResult :type "HitResult Structure (by ref)"))
  (bind _asjpcharacter (cast `JPCharacter` OtherActor))
  (bind _asjpplayer_controller (cast `JPPlayerController` (`Pawn.GetController` _asjpcharacter)))
  (bind _returnvalue (`BrunesMissionSystemInterface.GetMissionManager` _asjpplayer_controller))
  (bind _returnvalue_2 (`BruMissionManager.ActivateMission` _returnvalue (`self.MissionClass`)))
  (`/Engine/EditorBlueprintResources/StandardMacros.IsValid` _returnvalue_2
    (:`Is Valid`
      (`BruMissionMetaData.ActivateTask` _returnvalue_2 (`self.MisionTaskClass`) true))
    (:`Is Not Valid`
      (bind _returnvalue_3 (`BruMissionManager.FindActiveMissionByClass` _returnvalue (`self.MissionClass`)))
      (`BruMissionMetaData.ActivateTask` _returnvalue_3 (`self.MisionTaskClass`) true)))
  (`self.K2_DestroyActor`))

(fn `UserConstructionScript`)